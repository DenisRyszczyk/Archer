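; BP_ClickableMenuSkeleton is a skeleton actor that reacts to mouse clicks, likely as menu scenery.
; BeginPlay enables click events on the player controller, and clicking the capsule plays a death montage on the skeletal mesh.
; That click also reveals a static mesh, activates a Niagara effect, destroys the capsule so it cannot retrigger, and runs a timeline lerping the skeleton to the LandLoc position.
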(event `self.ReceiveBeginPlay`
  (set `PlayerController.bEnableClickEvents` true (`GameplayStatics.GetPlayerController` 0)))

(event `self.Capsule.OnClicked`
  (params (TouchedComponent :type "PrimitiveComponent Object Reference") (ButtonPressed :type "Key Structure"))
  (`|PlayMontage` (`self.SkeletalMesh`) "/Game/UndeadPack/SkeletonEnemy/Animations/AM_Skeleton_Death.AM_Skeleton_Death"
    (:`then`
      (`SceneComponent.SetVisibility` (`self.StaticMesh`) true false)
      (`ActorComponent.Activate` (`self.Niagara`) false)
      (`ActorComponent.K2_DestroyComponent` (`self.Capsule`))
      (bind (_direction _newtrack_0) (`Timeline|Timeline` :!via `PlayFromStart`)
        (:`Update`
          (`SceneComponent.K2_SetRelativeLocation` (`self.SkeletalMesh`) (`KismetMathLibrary.VLerp` (0.0 0.0 0.0) (`SceneComponent.RelativeLocation` (`self.LandLoc`)) _newtrack_0) false false))))))

(fn `UserConstructionScript`)