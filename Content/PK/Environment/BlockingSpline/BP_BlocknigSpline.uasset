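; Spline-based blocking actor that builds a segmented mesh along its spline and feeds the player's position to materials.
; The Construction Script adds spline mesh components at fixed intervals scaled by actor X scale, clamping tangents to the section length to fit each segment to the curve.
; Every Tick writes the first player character's location into the MPC_BlockVolume material parameter collection as PlayerLocation.
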(event `self.ReceiveTick`
  (params (DeltaSeconds :type "Float (single-precision)"))
  (bind _returnvalue (`GameplayStatics.GetPlayerCharacter` 0))
  (bind (_returnvalue_x _returnvalue_y _returnvalue_z) (`KismetMathLibrary.BreakVector` (`self.K2_GetActorLocation` _returnvalue)))
  (`/Engine/EditorBlueprintResources/StandardMacros.IsValid` _returnvalue
    (:`Is Valid`
      (`KismetMaterialLibrary.SetVectorParameterValue` "/Game/PK/Environment/BlockingSpline/MPC_BlockVolume.MPC_BlockVolume" "PlayerLocation" (make `LinearColor` _returnvalue_x _returnvalue_y _returnvalue_z 1.0)))))

(fn `UserConstructionScript`
  (locals (L_Index :type Integer))
  (bind _returnvalue_x (`KismetMathLibrary.BreakVector` (`self.GetActorScale3D`)))
  (set `self.Section Length` (* 400.0 _returnvalue_x))
  (for _index (range (+ (`KismetMathLibrary.FTrunc` (/ (`SplineComponent.GetSplineLength` (`self.Spline`)) (`self.Section Length`))) 1))
    (set `local.L_Index` _index)
    (bind _returnvalue (`AddComponent|NODE_AddSplineMeshComponent-0`))
    (`SplineMeshComponent.SetStartAndEnd` _returnvalue (`SplineComponent.GetLocationAtDistanceAlongSpline` (`self.Spline`) (* (`self.Section Length`) (`local.L_Index`)) "Local") (`KismetMathLibrary.ClampVectorSize` (`SplineComponent.GetTangentAtDistanceAlongSpline` (`self.Spline`) (* (`self.Section Length`) (`local.L_Index`)) "Local") 0.0 (`self.Section Length`)) (`SplineComponent.GetLocationAtDistanceAlongSpline` (`self.Spline`) (* (`self.Section Length`) (+ (`local.L_Index`) 1)) "Local") (`KismetMathLibrary.ClampVectorSize` (`SplineComponent.GetTangentAtDistanceAlongSpline` (`self.Spline`) (* (`self.Section Length`) (+ (`local.L_Index`) 1)) "Local") 0.0 (`self.Section Length`)) true)))