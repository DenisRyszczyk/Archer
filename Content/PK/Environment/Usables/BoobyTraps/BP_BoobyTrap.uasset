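; BP_BoobyTrap is a placed explosive trap that detonates when a living enemy walks into it.
; It spawns a surface ability particle effect on BeginPlay, then waits for a BP_Enemy to overlap its trigger Sphere.
; On trigger, it applies Damage to every BP_Enemy inside the separate DamageSphere, spawns a grenade explosion effect, plays a distance-based camera shake and destroys itself.
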(event `self.ReceiveBeginPlay`
  (`NiagaraFunctionLibrary.SpawnSystemAtLocation` "/Game/A_Surface_Footstep/Niagara_FX/ParticleSystems/PSN_SpecialABility_Surface.PSN_SpecialAbility_Surface" (`self.K2_GetActorLocation`)))

(event `self.Sphere.OnComponentBeginOverlap`
  (params (OverlappedComponent :type "PrimitiveComponent Object Reference") (OtherActor :type "Actor Object Reference") (OtherComp :type "PrimitiveComponent Object Reference") (OtherBodyIndex :type Integer) (bFromSweep :type Boolean) (SweepResult :type "HitResult Structure (by ref)"))
  (bind _asbp_enemy (cast `/Game/PK/Characters/Enemies/BP_Enemy` OtherActor))
  (if (not (`Enemy.IsDead` _asbp_enemy))
    (bind _output_get (set `self.Overlapping Actors` (`PrimitiveComponent.GetOverlappingActors` (`self.Damage Sphere`) "/Game/PK/Characters/Enemies/BP_Enemy.BP_Enemy_C")))
    (for _array_element _output_get
      (`GameplayStatics.ApplyDamage` _array_element (`self.Damage`)))
    (`NiagaraFunctionLibrary.SpawnSystemAtLocation` "/Game/Realistic_Starter_VFX_Pack_Niagara/Niagara/Explosion/NS_Explosion_Grenade.NS_Explosion_Grenade" (`self.K2_GetActorLocation`))
    (`GameplayStatics.PlayWorldCameraShake` "/Game/PK/Environment/Usables/BoobyTraps/CS_BoobyExplosion.CS_BoobyExplosion_C" (`self.K2_GetActorLocation`) 1000.0 2000.0 1.0 true)
    (`self.K2_DestroyActor`)))

(fn `UserConstructionScript`)