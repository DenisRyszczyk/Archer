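; BP_HealthPoint_1 is a health pickup that restores HP to the player character.
; It overrides a pickup condition that passes only while the player's current HP differs from their health slot count, so it is not collected at full health.
; Its ApplyEffect event casts player 0's character to BP_PlayerCharacter and calls AddHP with the AddedHP amount.
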(event `self.ApplyEffect`
  (bind _asbp_player_character (cast `/Game/PK/Characters/PlayerCharacter/BP_PlayerCharacter` (`GameplayStatics.GetPlayerCharacter` 0)))
  (`PlayerCharacter.AddHP` _asbp_player_character (`self.Added HP`)))

(fn `PickupConditionMet`
  (params (PlayerActor :type "Actor Object Reference"))
  (returns (ReturnValue :type Boolean))
  (bind _asbp_player_character (cast `/Game/PK/Characters/PlayerCharacter/BP_PlayerCharacter` PlayerActor))
  (return (not (== (`PlayerCharacter.CurrentHP` _asbp_player_character) (`PlayerCharacter.HealthSlots` _asbp_player_character)))))

(fn `UserConstructionScript`
  (`parent.UserConstructionScript`))