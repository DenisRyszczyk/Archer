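; BP_BoobyTrapBuff is a usable buff that grants or upgrades the player's booby trap placing ability.
; Its ApplyEffect event looks up the AC_BoobyTraps component on player character 0.
; If present, it cuts the PlacingRate by 20 percent, compounding with each application, and reruns the timer.
; Otherwise it adds the component to the character and starts its timer.
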(event `self.ApplyEffect`
  (bind _asbp_player_character (cast `/Game/PK/Characters/PlayerCharacter/BP_PlayerCharacter` (`GameplayStatics.GetPlayerCharacter` 0)))
  (bind _returnvalue (`self.GetComponentByClass` _asbp_player_character "/Game/PK/Environment/Usables/BoobyTraps/AC_BoobyTraps.AC_BoobyTraps_C"))
  (`/Engine/EditorBlueprintResources/StandardMacros.IsValid` _returnvalue
    (:`Is Valid`
      (bind _placing_rate (`/Game/PK/Environment/Usables/BoobyTraps/AC_BoobyTraps.Placing Rate` _returnvalue))
      (set `/Game/PK/Environment/Usables/BoobyTraps/AC_BoobyTraps.Placing Rate` (- _placing_rate (* _placing_rate 0.2)) _returnvalue)
      (`/Game/PK/Environment/Usables/BoobyTraps/AC_BoobyTraps.RunTimer` _returnvalue))
    (:`Is Not Valid`
      (bind _returnvalue_2 (`AddComponent|NODE_AddAC_BoobyTraps-0` :`self` _asbp_player_character))
      (`/Game/PK/Environment/Usables/BoobyTraps/AC_BoobyTraps.RunTimer` _returnvalue_2))))

(fn `UserConstructionScript`
  (`parent.UserConstructionScript`))