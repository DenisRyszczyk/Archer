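; BP_GoldPickup is a pickup that adds its GoldWorth to the player character's gold when its effect is applied.
; On BeginPlay, a Jump timeline tosses it from its spawn point to a random nearby XY offset, with a separate alpha driving height.
; When the toss finishes, it enables HoveringAndRotating.
; The construction script gives the mesh a random yaw rotation.
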(event `self.ReceiveBeginPlay`
  (bind (_spawn_loc_x _spawn_loc_y _spawn_loc_z) (`KismetMathLibrary.BreakVector` (`self.Spawn Loc`)))
  (`parent.ReceiveBeginPlay`)
  (set `self.Spawn Loc` (`self.K2_GetActorLocation`))
  (set `self.Random X` (`KismetMathLibrary.RandomFloatInRange` -120.0 120.0))
  (set `self.Randm Y` (`KismetMathLibrary.RandomFloatInRange` -120.0 120.0))
  (bind (_direction _height_alpha _distance_alpha) (`Timeline|Jump` :!via `PlayFromStart`)
    (:`Update`
      (bind (_returnvalue_x _returnvalue_y) (`KismetMathLibrary.BreakVector` (`KismetMathLibrary.VLerp` (`KismetMathLibrary.MakeVector` _spawn_loc_x _spawn_loc_y) (`KismetMathLibrary.MakeVector` (+ _spawn_loc_x (`self.Random X`)) (+ _spawn_loc_y (`self.Randm Y`))) _distance_alpha)))
      (`self.K2_SetActorLocation` (`KismetMathLibrary.MakeVector` _returnvalue_x _returnvalue_y (`KismetMathLibrary.Lerp` _spawn_loc_z (+ _spawn_loc_z 100.0) _height_alpha))))
    (:`Finished`
      (set `self.bHoveringAndRotating` true))))

(event `self.ApplyEffect`
  (bind _asbp_player_character (cast `/Game/PK/Characters/PlayerCharacter/BP_PlayerCharacter` (`GameplayStatics.GetPlayerCharacter` 0)))
  (`PlayerCharacter.AddGold` _asbp_player_character (`self.Gold Worth`)))

(fn `UserConstructionScript`
  (`parent.UserConstructionScript`)
  (`SceneComponent.K2_AddRelativeRotation` (`self.StaticMesh`) (`KismetMathLibrary.MakeRotator` 0.0 0.0 (`KismetMathLibrary.RandomFloatInRange` 100.0 300.0)) false false))