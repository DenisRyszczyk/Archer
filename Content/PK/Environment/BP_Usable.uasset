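; BP_Usable is a data-driven environment actor that shows a static mesh and a price defined by a data table row.
; The construction script looks up the Row handle and applies that row's mesh to the StaticMesh component.
; GetPrice reads the price from the same row, falling back to a very high placeholder when the row is missing.
; Tick draws that price as a debug string at the actor's location.
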(event `self.ReceiveTick`
  (params (DeltaSeconds :type "Float (single-precision)"))
  (`KismetSystemLibrary.DrawDebugString` (`self.K2_GetActorLocation`) (`KismetStringLibrary.Concat_StrStr` "Price: " (`KismetStringLibrary.Conv_IntToString` (`self.GetPrice`))) null))

(fn `GetPrice`
  (returns (ReturnValue :type Integer))
  (bind (_row_datatable _row_rowname) (break `DataTableRowHandle` (`self.Row`)))
  (bind _returnvalue (`|GetDataTableRow` _row_datatable _row_rowname)
    (:`then`
      (return (`.Price` (break `UsableData` _returnvalue))))
    (:`RowNotFound`
      (return 99999))))

(fn `UserConstructionScript`
  (bind (_datatable _rowname) (break `DataTableRowHandle` (`self.Row`)))
  (bind _returnvalue (`|GetDataTableRow` _datatable _rowname)
    (:`then`
      (`StaticMeshComponent.SetStaticMesh` (`self.StaticMesh`) (`.Mesh` (break `UsableData` _returnvalue))))))