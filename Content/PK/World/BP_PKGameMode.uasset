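; Game mode for PK that runs wave-based spawning, tracking the current wave and its spawners.
; On BeginPlay it calls GatherAllSpawners, EndWave and RemoveBuffs, whose logic is defined outside this graph.
; Tick prints a debug readout of the wave number, finished spawner count and spawners involved in the current wave.
; Disconnected debug snippets for printing user graphics settings and spawnable buff classes remain in the graph but never run.
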(event `self.ReceiveTick`
  (params (DeltaSeconds :type "Float (single-precision)"))
  ;[1 1 1] Debug wave info
  (`KismetSystemLibrary.PrintText` (`|FormatText` "Wave: {W} \nFinished spawners: {E} \nInvolved spawners: {O}" (`self.Wave`) (`self.FinishedSpawners`) (`KismetArrayLibrary.Array_Length` (`self.SpawnersInvlovedInCurrentWave`))) true true (struct :`G` 0.66 :`B` 1.0 :`A` 1.0) 0.0))

(event `self.ReceiveBeginPlay`
  (`self.GatherAllSpawners`)
  (`self.EndWave`)
  (`self.RemoveBuffs`))

(fn `UserConstructionScript`)