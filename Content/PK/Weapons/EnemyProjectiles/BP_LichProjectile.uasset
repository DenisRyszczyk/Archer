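; BP_LichProjectile is an enemy projectile, named for the Lich, that launches at a preset velocity and explodes.
; It explodes when its ProjectileMovement stops or when it takes any damage, so it can be shot down, and a BP_Arrow that hits it is destroyed too.
; The explosion spawns an effect, damages player characters overlapping its DamageSphere and destroys the projectile.
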(event `self.ReceiveBeginPlay`
  (set `MovementComponent.Velocity` (`self.Launch Velocity`) (`self.ProjectileMovement`)))

(event `Explode`
  (`NiagaraFunctionLibrary.SpawnSystemAtLocation` "/Game/Realistic_Starter_VFX_Pack_Niagara/Niagara/Explosion/NS_Explosion_C4.NS_Explosion_C4" (`self.K2_GetActorLocation`))
  (for _array_element (`PrimitiveComponent.GetOverlappingActors` (`self.Damage Sphere`) "/Game/PK/Characters/PlayerCharacter/BP_PlayerCharacter.BP_PlayerCharacter_C")
    (`GameplayStatics.ApplyDamage` _array_element 1.0 null self))
  (`self.K2_DestroyActor`))

(event `self.ProjectileMovement.OnProjectileStop`
  (params (ImpactResult :type "HitResult Structure (by ref)"))
  (`self.Explode`))

(event `self.ReceiveAnyDamage`
  (params (Damage :type "Float (single-precision)") (DamageType :type "DamageType Object Reference") (InstigatedBy :type "Controller Object Reference") (DamageCauser :type "Actor Object Reference"))
  (`self.Explode`)
  (bind _asbp_arrow (cast `/Game/PK/Weapons/Bow/Arrows/BP_Arrow` DamageCauser))
  (`self.K2_DestroyActor` _asbp_arrow))

(fn `UserConstructionScript`)