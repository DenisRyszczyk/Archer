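; Actor component for a bow arrow effect that freezes the owning BP_Enemy for a set Duration.
; On BeginPlay it pauses a living enemy's mesh animations, while Tick stops its character movement every frame.
; A retriggerable delay then unpauses animations and destroys the component.
; Non-enemy owners destroy it immediately; on already-dead enemies it is never removed and keeps halting movement.
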(event `self.ReceiveBeginPlay`
  (bind _asbp_enemy (cast `/Game/PK/Characters/Enemies/BP_Enemy` (`self.GetOwner`))
    (:`then`
      (bind _output_get (set `self.As BP Enemy` _asbp_enemy))
      (if (not (`Enemy.IsDead` _output_get))
        (`self.Freeze Actor`)))
    (:`CastFailed`
      (`self.K2_DestroyComponent`))))

(event `Freeze Actor`
  (set `SkeletalMeshComponent.bPauseAnims` true (`Character.Mesh` (`self.As BP Enemy`)))
  (`KismetSystemLibrary.RetriggerableDelay` (`self.Duration`))
  (`self.Finish freeze`))

(event `Finish freeze`
  (set `SkeletalMeshComponent.bPauseAnims` false (`Character.Mesh` (`self.As BP Enemy`)))
  (`self.K2_DestroyComponent`))

(event `self.ReceiveTick`
  (params (DeltaSeconds :type "Float (single-precision)"))
  (`MovementComponent.StopMovementImmediately` (`Character.CharacterMovement` (`self.As BP Enemy`))))