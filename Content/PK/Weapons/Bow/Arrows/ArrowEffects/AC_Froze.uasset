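; AC_Froze is an actor component from the bow's arrow effects that freezes a living BP_Enemy owner for a set duration.
; On BeginPlay it pauses the mesh animations and zeroes the enemy's custom time dilation, then restores both and destroys itself after a retriggerable delay.
; It removes itself immediately on non-enemy owners and draws a "Froze" debug label above the owner every tick.
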(event `self.ReceiveTick`
  (params (DeltaSeconds :type "Float (single-precision)"))
  (`KismetSystemLibrary.DrawDebugString` (+ (`Actor.K2_GetActorLocation` (`self.GetOwner`)) (0.0 0.0 50.0)) "Froze" null (struct :`G` 0.432318 :`B` 1.0 :`A` 1.0)))

(event `self.ReceiveBeginPlay`
  (bind _asbp_enemy (cast `/Game/PK/Characters/Enemies/BP_Enemy` (`self.GetOwner`))
    (:`then`
      (bind _output_get (set `self.As BP Enemy` _asbp_enemy))
      (if (not (`Enemy.IsDead` _output_get))
        (`self.Freeze Actor`)))
    (:`CastFailed`
      (`self.K2_DestroyComponent`))))

(event `Freeze Actor`
  (set `SkeletalMeshComponent.bPauseAnims` true (`Character.Mesh` (`self.As BP Enemy`)))
  (set `Actor.CustomTimeDilation` 0.0 (`self.As BP Enemy`))
  (`KismetSystemLibrary.RetriggerableDelay` (`self.Duration`))
  (`self.Finish freeze`))

(event `Finish freeze`
  (set `SkeletalMeshComponent.bPauseAnims` false (`Character.Mesh` (`self.As BP Enemy`)))
  (set `Actor.CustomTimeDilation` 1.0 (`self.As BP Enemy`))
  (`self.K2_DestroyComponent`))