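; Actor component for an on-fire arrow effect that deals damage over time to its owner.
; RunTimer restarts a looping damage timer and a retriggerable delay, so a repeat call refreshes the burn before the component destroys itself.
; Each damage tick also removes the component if the owner is a dead BP_Enemy or not a BP_Enemy at all.
; Tick draws a red "On Fire" debug label above the owner.
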(event `self.ReceiveTick`
  (params (DeltaSeconds :type "Float (single-precision)"))
  (`KismetSystemLibrary.DrawDebugString` (+ (`Actor.K2_GetActorLocation` (`self.GetOwner`)) (0.0 0.0 50.0)) "On Fire" null (struct :`R` 1.0 :`A` 1.0)))

(event `Run Timer`
  (`KismetSystemLibrary.K2_ClearAndInvalidateTimerHandle` (`self.Timer`))
  (bind _returnvalue (`KismetSystemLibrary.K2_SetTimerDelegate` (delegate `Damage Tick`) (`self.Interval time`) true))
  (set `self.Timer` _returnvalue)
  (`KismetSystemLibrary.RetriggerableDelay` (`self.Duration`))
  (`self.K2_DestroyComponent`))

(event `Damage Tick`
  (`GameplayStatics.ApplyDamage` (`self.GetOwner`) (`self.Damage on tick`))
  (bind _asbp_enemy (cast `/Game/PK/Characters/Enemies/BP_Enemy` (`self.GetOwner`))
    (:`then`
      (if (`Enemy.IsDead` _asbp_enemy)
        (`self.K2_DestroyComponent`)))
    (:`CastFailed`
      (`self.K2_DestroyComponent`))))