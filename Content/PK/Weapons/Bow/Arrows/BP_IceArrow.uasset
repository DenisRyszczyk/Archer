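; BP_IceArrow is a bow arrow that freezes the actor it hits.
; It implements the ApplyEffecttoHitActor event, which calls FreezeActor on the target's existing AC_Frozen component or adds that component when it is missing.
; In parallel, a two-second delay deactivates the arrow's Niagara effect.
; The construction script only calls the parent's, so this child class supplies just the ice effect.
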(event `self.ApplyEffectToHitActor`
  (params (ActorToApplyEffect :type "Actor Object Reference"))
  (bind _returnvalue (`self.GetComponentByClass` ActorToApplyEffect "/Game/PK/Weapons/Bow/Arrows/ArrowEffects/AC_Frozen.AC_Frozen_C"))
  (`/Engine/EditorBlueprintResources/StandardMacros.IsValid` ActorToApplyEffect
    (:`Is Valid`
      (`|ExecutionSequence`
        (:`then_0`
          (`KismetSystemLibrary.Delay` 2.0)
          (`ActorComponent.Deactivate` (`self.Niagara`)))
        (:`then_1`
          (`/Engine/EditorBlueprintResources/StandardMacros.IsValid` _returnvalue
            (:`Is Valid`
              (`/Game/PK/Weapons/Bow/Arrows/ArrowEffects/AC_Frozen.Freeze Actor` _returnvalue))
            (:`Is Not Valid`
              (`AddComponent|NODE_AddAC_Froze-0` :`self` ActorToApplyEffect))))))))

(fn `UserConstructionScript`
  (`parent.UserConstructionScript`))