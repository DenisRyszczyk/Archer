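; BP_FireArrow is a bow arrow Blueprint that sets the actor it hits on fire.
; Its ApplyEffecttoHitActor event reuses the target's AC_OnFire component or adds one if none exists, then starts that component's timer.
; The same event also shuts off the arrow's Niagara effect after a short delay.
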(event `self.ApplyEffectToHitActor`
  (params (ActorToApplyEffect :type "Actor Object Reference"))
  (bind _returnvalue (`self.GetComponentByClass` ActorToApplyEffect "/Game/PK/Weapons/Bow/Arrows/ArrowEffects/AC_OnFire.AC_OnFire_C"))
  (`|ExecutionSequence`
    (:`then_0`
      (`KismetSystemLibrary.Delay` 5.0)
      (`ActorComponent.Deactivate` (`self.Niagara`)))
    (:`then_1`
      (`/Engine/EditorBlueprintResources/StandardMacros.IsValid` _returnvalue
        (:`Is Valid`
          (`/Game/PK/Weapons/Bow/Arrows/ArrowEffects/AC_OnFire.Run Timer` _returnvalue))
        (:`Is Not Valid`
          (bind _returnvalue_2 (`AddComponent|NODE_AddAC_OnFire-0` :`self` ActorToApplyEffect))
          (`/Engine/EditorBlueprintResources/StandardMacros.IsValid` _returnvalue_2
            (:`Is Valid`
              (`/Game/PK/Weapons/Bow/Arrows/ArrowEffects/AC_OnFire.Run Timer` _returnvalue_2))))))))

(fn `UserConstructionScript`
  (`parent.UserConstructionScript`))