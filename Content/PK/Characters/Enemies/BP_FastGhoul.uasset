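; BP_FastGhoul is an enemy character that chases the first player and attacks at close range.
; Each Tick it feeds movement input blended from its normalized velocity toward the player's direction, steering directly without pathfinding.
; Walk speed is remapped from player distance, so the ghoul speeds up as it closes in.
; Within attack range it calls PerformAttack, which is not defined in this Blueprint, on every Tick.
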(event `self.ReceiveBeginPlay`
  (`parent.ReceiveBeginPlay`))

(event `self.ReceiveTick`
  (params (DeltaSeconds :type "Float (single-precision)"))
  (`parent.ReceiveTick` DeltaSeconds)
  (`self.AddMovementInput` (`KismetMathLibrary.VInterpTo` (`KismetMathLibrary.Normal` (`self.GetVelocity`)) (`KismetMathLibrary.GetForwardVector` (`KismetMathLibrary.FindLookAtRotation` (`self.K2_GetActorLocation`) (`self.K2_GetActorLocation` (`GameplayStatics.GetPlayerCharacter` 0)))) (`GameplayStatics.GetWorldDeltaSeconds`) 20.0))
  (set `CharacterMovementComponent.MaxWalkSpeed` (`KismetMathLibrary.MapRangeClamped` (`self.GetDistanceTo` (`GameplayStatics.GetPlayerCharacter` 0)) 100.0 1000.0 600.0 450.0) (`self.CharacterMovement`))
  (if (< (`self.GetDistanceTo` (`GameplayStatics.GetPlayerCharacter` 0)) 350.0)
    (`self.PerformAttack`)))

(fn `UserConstructionScript`
  (`parent.UserConstructionScript`))