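; BP_Enemy is an enemy Blueprint that drives an emissive material effect on its mesh whenever it is hit.
; On BeginPlay it creates a dynamic material instance at the configured material index, caches the initial value of the emissive scalar parameter and binds to OnHit.
; Each hit restarts a Timeline whose track lerps that parameter between the cached value and a fixed high intensity.
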(event `self.ReceiveBeginPlay`
  (`self.CreateMeshDynamicMatInstance`)
  (`self.Get Initial Emissive Power Scalar Parameter`)
  (add `self.OnHit` (delegate `OnHit_Event`)))

(event `OnHit_Event`
  (bind _dynamic_mat (`self.Dynamic Mat`)
    (:`then`
      (bind (_direction _newtrack_0) (`Timeline|Timeline` :!via `PlayFromStart`)
        (:`Update`
          (`MaterialInstanceDynamic.SetScalarParameterValue` _dynamic_mat (`self.Emissive Parameter Name`) (`KismetMathLibrary.Lerp` (`self.Initial Emissive Parameter`) 2000.0 _newtrack_0)))))
    (:`else`)))

(fn `CreateMeshDynamicMatInstance`
  (bind _returnvalue (`PrimitiveComponent.CreateDynamicMaterialInstance` (`self.Mesh`) (`self.Emissive Mat Index`) null "None"))
  (set `self.Dynamic Mat` _returnvalue))

(fn `Get Initial Emissive Power Scalar Parameter`
  (bind _dynamic_mat (`self.Dynamic Mat`)
    (:`then`
      (bind _returnvalue (`MaterialInstanceDynamic.K2_GetScalarParameterValue` _dynamic_mat (`self.Emissive Parameter Name`)))
      (set `self.Initial Emissive Parameter` _returnvalue))
    (:`else`)))

(fn `UserConstructionScript`)