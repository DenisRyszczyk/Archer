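; BP_Skeleton is a skeleton enemy character whose AI runs on the BT_Basic behavior tree, started on its AI controller at BeginPlay.
; Every tick it remaps its distance to player 0 into a clamped max walk speed, so it moves faster when far from the player and slows as it gets close.
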(event `self.ReceiveBeginPlay`
  (`parent.ReceiveBeginPlay`)
  (`AIController.RunBehaviorTree` (`AIBlueprintHelperLibrary.GetAIController` self) "/Game/PK/AI/BTs/BT_Basic.BT_Basic"))

(event `self.ReceiveTick`
  (params (DeltaSeconds :type "Float (single-precision)"))
  (`parent.ReceiveTick` DeltaSeconds)
  (set `CharacterMovementComponent.MaxWalkSpeed` (`KismetMathLibrary.MapRangeClamped` (`self.GetDistanceTo` (`GameplayStatics.GetPlayerCharacter` 0)) 300.0 1000.0 240.0 500.0) (`self.CharacterMovement`)))

(fn `UserConstructionScript`
  (`parent.UserConstructionScript`))