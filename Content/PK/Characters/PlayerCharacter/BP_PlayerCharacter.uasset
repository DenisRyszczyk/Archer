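; Player character Blueprint for a wave-based game with gold, pulling and health slots.
; BeginPlay sets up Enhanced Input, cursor, fixed-rotation camera boom and HUD.
; Input drives movement, toggles Pulling status, opens the menu map and asks BP_PKGameMode to start waves early.
; Debug keys grant gold and health slots, toggle invincibility, spawn or damage enemies; Tick draws status and velocity, while the construction script makes modular body meshes follow the main mesh's pose.
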(event `self.ReceiveBeginPlay`
  (bind _returnvalue (pcsubsystem `EnhancedInputLocalPlayerSubsystem` (`GameplayStatics.GetPlayerController` 0)))
  (`/Engine/EditorBlueprintResources/StandardMacros.IsValid` _returnvalue
    (:`Is Valid`
      (`EnhancedInputSubsystemInterface.AddMappingContext` _returnvalue "/Game/PK/Input/IMC_PlayerInput.IMC_PlayerInput" 0 (struct))
      (set `PlayerController.bShowMouseCursor` true (`GameplayStatics.GetPlayerController` 0))
      (set `SceneComponent.bAbsoluteRotation` true (`self.SpringArm`))
      (bind _returnvalue_2 (`|CreateWidget` "/Game/PK/UI/HUD/W_HUD.W_HUD_C" null self))
      (`UserWidget.AddToViewport` _returnvalue_2 0))))

(event `self.ReceiveTick`
  (params (DeltaSeconds :type "Float (single-precision)"))
  (bind _returnvalue (- (`self.K2_GetActorLocation`) (0.0 0.0 50.0)))
  (`KismetSystemLibrary.DrawDebugString` (`self.K2_GetActorLocation`) (`KismetStringLibrary.Concat_StrStr` "Status: " (`|GetEnumeratorNameAsString` (`self.PlayerStatus`)) " \n" "Invincible: " (`KismetStringLibrary.Conv_BoolToString` (`self.bInvincible`)) " \n" "Gold: " (`KismetStringLibrary.Conv_IntToString` (`self.Gold`))) null)
  (`KismetSystemLibrary.DrawDebugArrow` _returnvalue (+ _returnvalue (/ (`self.GetVelocity`) 5.0)) 0.0 (struct :`R` 0.250158 :`G` 0.806952 :`B` 0.323143 :`A` 1.0)))

(event `EnhancedInput|/Game/PK/Input/IA_Movement`
  (params (ActionValue :type "Vector2D Structure") (ElapsedSeconds :type "Float (double-precision)") (TriggeredSeconds :type "Float (double-precision)") (InputAction :type "InputAction Object Reference" :default "/Game/PK/Input/IA_Movement.IA_Movement"))
  (:`Triggered`
    (`self.HandleMovementInput` ActionValue_X ActionValue_Y)))

(event `EnhancedInput|/Game/PK/Input/IA_Pull`
  (params (ActionValue :type Boolean) (ElapsedSeconds :type "Float (double-precision)") (TriggeredSeconds :type "Float (double-precision)") (InputAction :type "InputAction Object Reference" :default "/Game/PK/Input/IA_Pull.IA_Pull"))
  (:`Started`
    (`self.ChangeStatus` "EPS_Pulling"))
  (:`Canceled`
    (`self.ChangeStatus` "EPS_Normal" :!label _label))
  (:`Completed`
    (goto _label)))

(event `Key|E`
  (params (Key :type "Key Structure"))
  (:`Pressed`
    (`self.AddGold` 100)))

(event `EnhancedInput|/Game/PK/Input/IA_Escape`
  (params (ActionValue :type Boolean) (ElapsedSeconds :type "Float (double-precision)") (TriggeredSeconds :type "Float (double-precision)") (InputAction :type "InputAction Object Reference" :default "/Game/PK/Input/IA_Escape.IA_Escape"))
  (:`Started`
    (`GameplayStatics.OpenLevelBySoftObjectPtr` "/Game/PK/Levels/Map_Menu.Map_Menu")))

(event `Key|F`
  (params (Key :type "Key Structure"))
  (:`Pressed`
    (bind _isa (`/Engine/EditorBlueprintResources/StandardMacros.FlipFlop`)
      (:`A`
        (set `self.bInvincible` _isa))
      (:`B`
        (set `self.bInvincible` false)))))

(event `EnhancedInput|/Game/PK/Input/IA_SkipWaiting`
  (params (ActionValue :type Boolean) (ElapsedSeconds :type "Float (double-precision)") (TriggeredSeconds :type "Float (double-precision)") (InputAction :type "InputAction Object Reference" :default "/Game/PK/Input/IA_SkipWaiting.IA_SkipWaiting"))
  (:`Started`
    (bind _asbp_pkgame_mode (cast `/Game/PK/World/BP_PKGameMode` (`GameplayStatics.GetGameMode`)))
    (bind _returnvalue (`PKGameMode.CanStartWaveEarly` _asbp_pkgame_mode))
    (if _returnvalue
      (`PKGameMode.StartWave` _asbp_pkgame_mode))))

(event `Key|One`
  (params (Key :type "Key Structure"))
  (:`Pressed`
    (`|SpawnActorFromClass` "/Game/PK/Characters/Enemies/BP_BasicGhoul.BP_BasicGhoul_C" (`KismetMathLibrary.MakeTransform` (0.0 0.0 0.0)) "AdjustIfPossibleButAlwaysSpawn" "MultiplyWithRoot" null null)))

(event `Key|Two`
  (params (Key :type "Key Structure"))
  (:`Pressed`
    (`|SpawnActorFromClass` "/Game/PK/Characters/Enemies/BP_FastGhoul.BP_FastGhoul_C" (`KismetMathLibrary.MakeTransform` (0.0 0.0 0.0)) "AdjustIfPossibleButAlwaysSpawn" "MultiplyWithRoot" null null)))

(event `Key|Three`
  (params (Key :type "Key Structure"))
  (:`Pressed`
    (`|SpawnActorFromClass` "/Game/PK/Characters/Enemies/BP_Lich.BP_Lich_C" (`KismetMathLibrary.MakeTransform` (0.0 0.0 0.0)) "AdjustIfPossibleButAlwaysSpawn" "MultiplyWithRoot" null null)))

(event `Key|Four`
  (params (Key :type "Key Structure"))
  (:`Pressed`
    (`|SpawnActorFromClass` "/Game/PK/Characters/Enemies/BP_Skeleton.BP_Skeleton_C" (`KismetMathLibrary.MakeTransform` (0.0 0.0 0.0)) "AdjustIfPossibleButAlwaysSpawn" "MultiplyWithRoot" null null)))

(event `Key|R`
  (params (Key :type "Key Structure"))
  (:`Pressed`
    (bind _outactors (`GameplayStatics.GetAllActorsOfClass` "/Game/PK/Characters/Enemies/BP_Enemy.BP_Enemy_C"))
    (for _array_element _outactors
      (`GameplayStatics.ApplyDamage` _array_element 500.0))))

(event `Key|T`
  (params (Key :type "Key Structure"))
  (:`Pressed`
    (`self.AddHealthSlot` 1)))

(fn `UserConstructionScript`
  (`SkinnedMeshComponent.SetLeaderPoseComponent` (`self.SK_Body_Face`) (`self.Mesh`) false false)
  (`SkinnedMeshComponent.SetLeaderPoseComponent` (`self.SK_Casual_Hands`) (`self.Mesh`) false false)
  (`SkinnedMeshComponent.SetLeaderPoseComponent` (`self.SK_Casual_Legs`) (`self.Mesh`) false false))